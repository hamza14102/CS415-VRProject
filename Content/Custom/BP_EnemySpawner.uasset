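; BP_EnemySpawner is an actor that endlessly spawns BP_Barbarian_ enemies at its own transform, marked by a fire effect and sound on BeginPlay.
; SpawnEnemy waits a random delay scaled by Speed, spawns with collision adjustment or skips if blocked, then calls itself to loop.
; Tick lowers Speed by a fixed per-frame step down to a floor, so spawns grow more frequent at a framerate-dependent rate.
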(event Custom|Spawn%20Enemy
  (Utilities|FlowControl|Delay (* (Math|Random|RandomIntegerinRange 5 15) (Variables|Default|GetSpeed)))
  (Game|SpawnActorfromClass "/Game/Assets/Adventurers/Characters/Blueprints/BP_Barbarian_.BP_Barbarian__C" (Transformation|GetActorTransform) "AdjustIfPossibleButDontSpawnIfColliding" "MultiplyWithRoot" 0 0)
  (CallFunction|SpawnEnemy))

(event EventBeginPlay
  (bind _returnvalue (Transformation|GetActorLocation))
  (Effects|SpawnEmitteratLocation "/Game/StarterContent/Particles/P_Fire.P_Fire" _returnvalue)
  (Audio|SpawnSoundatLocation "/Game/VRTemplate/Audio/Fire01.Fire01" _returnvalue "0, 0, 0" 1.0 1.0 0.0 0 0)
  (CallFunction|SpawnEnemy))

(event Collision|EventActorBeginOverlap
  (params (OtherActor :type Actor%20Object%20Reference)))

(event EventTick
  (params (DeltaSeconds :type Float%20%28single-precision%29))
  (if (>= (- (Variables|Default|GetSpeed) 0.0001) 0.1)
    (Variables|Default|SetSpeed (- (Variables|Default|GetSpeed) 0.0001))))

(fn ConstructionScript)