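; BP_NewEneemy is an enemy Blueprint that wanders randomly; despite its name, ChasePlayer never references the player.
; From BeginPlay, ChasePlayer waits briefly, picks a nearby navigable point and issues AIMoveTo at the actor's current height.
; It re-calls itself from the move's immediate output, so retargeting follows the delay rather than arrival.
; Debug spheres mark position and destination, and printed messages report success or failure.
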(event Custom|ChasePlayer
  (bind _returnvalue (Transformation|GetActorLocation))
  (Utilities|FlowControl|Delay 3.0)
  (bind _randomlocation (Class|NavigationSystemV1|GetRandomLocationinNavigableRadius (Transformation|GetActorLocation) 5e+02 0 0))
  (AI|AIMoveTo 0 (Math|Vector|MakeVector (.x _randomlocation) (.y _randomlocation) (.z _returnvalue)) 0 1e+02 false
    (:then
      (Rendering|Debug|DrawDebugSphere (Transformation|GetActorLocation) 1e+02 12 "(R=1.000000,G=1.000000,B=1.000000,A=1.000000)" 3.0)
      (CallFunction|ChasePlayer)
      (Rendering|Debug|DrawDebugSphere (Math|Vector|MakeVector (.x _randomlocation) (.y _randomlocation) (.z _returnvalue)) 1e+02 12 "(R=1.000000,G=0.000000,B=0.000000,A=1.000000)" 3.0))
    (:OnSuccess
      (Development|PrintString "Reached Point"))
    (:OnFail
      (Development|PrintString "Could not reach"))))

(event EventBeginPlay
  (CallFunction|ChasePlayer))

(event Collision|EventActorBeginOverlap
  (params (OtherActor :type Actor%20Object%20Reference)))

(event EventTick
  (params (DeltaSeconds :type Float%20%28single-precision%29)))

(fn ConstructionScript)