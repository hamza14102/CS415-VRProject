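; BP_Barbarian_ is an enemy character that hurts and knocks back the first-person player on contact.
; A capsule overlap applies fixed damage and launches the player along the flattened, normalized direction away from the capsule, with a strong upward component, scaled by LaunchVelocity.
; After the hit it disables its own movement for a few seconds, then restores walking and calls RandomRoam.
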(event OnComponentBeginOverlap(Capsule)
  (params (OverlappedComponent :type Primitive%20Component%20Object%20Reference) (OtherActor :type Actor%20Object%20Reference) (OtherComp :type Primitive%20Component%20Object%20Reference) (OtherBodyIndex :type Integer) (bFromSweep :type Boolean) (SweepResult :type Hit%20Result%20Structure%20%28by%20ref%29))
  (bind _asbp_first_person_character (Utilities|Casting|CastToBP_FirstPersonCharacter OtherActor))
  (Utilities|FlowControl|Sequence
    (:then_0
      (Game|Damage|ApplyDamage _asbp_first_person_character 1e+01 0 self))
    (:then_1
      (Character|LaunchCharacter _asbp_first_person_character (* (Math|Vector|MakeVector (.x (Class|KismetMathLibrary|VectorNormal2D (Math|Vector|MakeVector (.x (Math|Vector|GetUnitDirection(Vector) (Transformation|GetWorldLocation (Variables|Default|GetCapsule)) (Transformation|GetActorLocation _asbp_first_person_character))) (.y (Math|Vector|GetUnitDirection(Vector) (Transformation|GetWorldLocation (Variables|Default|GetCapsule)) (Transformation|GetActorLocation _asbp_first_person_character))) 0.0) 0.0001)) (.y (Class|KismetMathLibrary|VectorNormal2D (Math|Vector|MakeVector (.x (Math|Vector|GetUnitDirection(Vector) (Transformation|GetWorldLocation (Variables|Default|GetCapsule)) (Transformation|GetActorLocation _asbp_first_person_character))) (.y (Math|Vector|GetUnitDirection(Vector) (Transformation|GetWorldLocation (Variables|Default|GetCapsule)) (Transformation|GetActorLocation _asbp_first_person_character))) 0.0) 0.0001)) 2.0) (Variables|Default|GetLaunch%20Velocity)) false false)
      (Pawn|Components|CharacterMovement|DisableMovement (Variables|Character|GetCharacterMovement))
      (Utilities|FlowControl|Delay 4.0)
      (Pawn|Components|CharacterMovement|SetMovementMode (Variables|Character|GetCharacterMovement) "MOVE_Walking" 0)
      (CallFunction|RandomRoam))))

(fn ConstructionScript
  (|CallParentFunction))