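; BP_Parent is an adventurer AI character that seeks gold bars and chases the player on sight.
; It loops a barbarian walk animation, while RandomRoam moves it to a GrabbableGoldBar found by class, repeating on success, rather than a random point.
; Pawn sensing plays a sound for any seen pawn and pursues the first-person character.
; A retriggerable delay clears CanSeeEnemy and resumes gold seeking shortly after sightings stop.
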(event OnSeePawn(PawnSensing)
  (params (Pawn :type Pawn%20Object%20Reference))
  (Utilities|FlowControl|Sequence
    (:then_0
      (Audio|PlaySound2D "/Game/Assets/Adventurers/Characters/Blueprints/Monster-Footsteps-A-www_fesliyanstudios_com.Monster-Footsteps-A-www_fesliyanstudios_com" 1.0 1.0 0.0 0 0))
    (:then_1
      (bind _asbp_first_person_character (Utilities|Casting|CastToBP_FirstPersonCharacter Pawn))
      (Utilities|FlowControl|Sequence
        (:then_0
          (Variables|Default|SetCanSeeEnemy true)
          (AI|AIMoveTo self "0, 0, 0" _asbp_first_person_character 5.0 false))
        (:then_1
          (Utilities|FlowControl|RetriggerableDelay 0.6)
          (Variables|Default|SetCanSeeEnemy false)
          (CallFunction|RandomRoam))))))

(event Custom|Random%20Roam
  (bind _returnvalue (Actor|GetActorOfClass "/Game/VRTemplate/Blueprints/GrabbableGoldBar.GrabbableGoldBar_C"))
  (AI|AIMoveTo self "0, 0, 0" _returnvalue 5.0 false
    (:OnSuccess
      (CallFunction|RandomRoam))))

(event EventBeginPlay
  (Utilities|FlowControl|Sequence
    (:then_0
      (Components|Animation|PlayAnimation (Variables|Character|GetMesh) "/Game/Assets/Adventurers/Characters/Barbarian/Barbarian_Anim_Walking_B.Barbarian_Anim_Walking_B" true))
    (:then_1
      (CallFunction|RandomRoam))))

(event Collision|EventActorBeginOverlap
  (params (OtherActor :type Actor%20Object%20Reference)))

(event EventTick
  (params (DeltaSeconds :type Float%20%28single-precision%29)))

(fn ConstructionScript)